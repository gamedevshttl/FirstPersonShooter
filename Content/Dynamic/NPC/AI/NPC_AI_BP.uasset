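; AI controller for guard NPCs that runs the GuardBehaviour tree on the PatrolData blackboard.
; AI perception updates react only to actors without the "Enemy" tag.
; A sensed actor becomes the blackboard enemy and turns on the PatrollinGuard2 pawn's aiming and shooting flags.
; Losing it clears the enemy, records the actor's location as last seen, and turns both flags off.
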(event OnTargetPerceptionUpdated(AIPerception)
  (params (Actor :type Actor%20Object%20Reference) (Stimulus :type AI%20Stimulus%20Structure))
  (bind _returnvalue (Pawn|GetControlledPawn))
  (bind _enemykey (Variables|Default|GetEnemyKey))
  (bind _blackboardcomp (Variables|Default|GetBlackboardComp))
  (bind _blackboardcomp_2 (Variables|Default|GetBlackboardComp))
  (bind _lastseenlocationkey (Variables|Default|GetLastSeenLocationKey))
  (if (not (Actor|ActorHasTag Actor "Enemy"))
    (if (.bSuccessfullySensed (Utilities|Struct|BreakAIStimulus Stimulus))
      (AI|Components|Blackboard|SetValueasObject _blackboardcomp _enemykey Actor)
      (AI|Components|Blackboard|ClearValue _blackboardcomp_2 _lastseenlocationkey)
      (bind _aspatrollin_guard_2 (Utilities|Casting|CastToPatrollinGuard2 _returnvalue))
      (Variables|/Game/Dynamic/NPC/Behaviour/PatrollinGuard2.PatrollinGuard2_C|SetAming _aspatrollin_guard_2 true)
      (Variables|/Game/Dynamic/NPC/Behaviour/PatrollinGuard2.PatrollinGuard2_C|SetShooting _aspatrollin_guard_2 true)
      (else
        (AI|Components|Blackboard|ClearValue _blackboardcomp _enemykey)
        (AI|Components|Blackboard|SetValueasVector _blackboardcomp_2 _lastseenlocationkey (Transformation|GetActorLocation Actor))
        (bind _aspatrollin_guard_2_2 (Utilities|Casting|CastToPatrollinGuard2 _returnvalue))
        (Variables|/Game/Dynamic/NPC/Behaviour/PatrollinGuard2.PatrollinGuard2_C|SetAming _aspatrollin_guard_2_2 false)
        (Variables|/Game/Dynamic/NPC/Behaviour/PatrollinGuard2.PatrollinGuard2_C|SetShooting _aspatrollin_guard_2_2 false)))))

(event EventBeginPlay
  (bind _blackboardcomponent (Class|AIController|UseBlackboard "/Game/Dynamic/NPC/AI/PatrolData.PatrolData"))
  (AI|RunBehaviorTree "/Game/Dynamic/NPC/AI/GuardBehaviour.GuardBehaviour")
  (Variables|Default|SetBlackboardComp _blackboardcomponent))

(fn ConstructionScript)