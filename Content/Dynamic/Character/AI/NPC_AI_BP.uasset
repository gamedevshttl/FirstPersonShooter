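; NPC AI controller that sets up the patrol blackboard and runs the guard behaviour tree on BeginPlay.
; AI perception treats any actor without the "Enemy" tag as a target, storing it in the enemy key when sensed.
; When sensing is lost, it clears that key and records the actor's current location as last seen.
; Unconnected leftover nodes toggle the controlled character's aiming and shooting flags but never run.
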(event OnTargetPerceptionUpdated(AIPerception)
  (params (Actor :type Actor%20Object%20Reference) (Stimulus :type AI%20Stimulus%20Structure))
  (bind _enemykey (Variables|Default|GetEnemyKey))
  (bind _blackboardcomp (Variables|Default|GetBlackboardComp))
  (bind _blackboardcomp_2 (Variables|Default|GetBlackboardComp))
  (bind _lastseenlocationkey (Variables|Default|GetLastSeenLocationKey))
  (if (not (Actor|ActorHasTag Actor "Enemy"))
    (if (.bSuccessfullySensed (Utilities|Struct|BreakAIStimulus Stimulus))
      (AI|Components|Blackboard|SetValueasObject _blackboardcomp _enemykey Actor)
      (AI|Components|Blackboard|ClearValue _blackboardcomp_2 _lastseenlocationkey)
      (else
        (AI|Components|Blackboard|ClearValue _blackboardcomp _enemykey)
        (AI|Components|Blackboard|SetValueasVector _blackboardcomp_2 _lastseenlocationkey (Transformation|GetActorLocation Actor))))))

(event EventBeginPlay
  (bind _blackboardcomponent (Class|AIController|UseBlackboard "/Game/Dynamic/Character/AI/PatrolData.PatrolData"))
  (AI|RunBehaviorTree "/Game/Dynamic/Character/AI/GuardBehaviour.GuardBehaviour")
  (Variables|Default|SetBlackboardComp _blackboardcomponent))

(fn ConstructionScript)